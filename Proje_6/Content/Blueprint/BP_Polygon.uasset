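; BP_Polygon is an actor that positions a fourth cube at the center point of three other cubes.
; On BeginPlay it averages the world locations of Cube1, Cube2 and Cube3 and moves Cube4 to that centroid.
; The placement runs once, without sweep or teleport, and the construction script is empty.
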(event EventBeginPlay
  ;[1 1 1] Kübün orta noktasını bulma
  (Transformation|SetWorldLocation (Variables|Default|GetCube4) (/ (+ (+ (Transformation|GetWorldLocation (Variables|Default|GetCube2)) (Transformation|GetWorldLocation (Variables|Default|GetCube1))) (Transformation|GetWorldLocation (Variables|Default|GetCube3))) "3.000000,3.000000,3.000000") false false))

(fn ConstructionScript)